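; Battle character with an Active Time Battle gauge, timed status effects and healing, with empty UI and notify functions.
; Tick fills the gauge through a Gate that closes when full until RestartATB reopens it.
; Shell, Haste/Slow and Regen count down per tick, not by delta time; Regen periodically calls Healed, which caps at MaxHP.
; Regen expiry clears HasteEnabled instead of RegenEnabled, and Slow expiry halves the fill rate like Haste.
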(event Custom|RestartATB
  (Development|PrintString "Restart ATB")
  (Variables|Default|SetCurrent%20Filled 0.0)
  (Utilities|FlowControl|Gate false) ; enters at Open
)

(event Custom|Healed
  (params (Amount%20Healed :type Integer) (Reviving? :type Boolean))
  (Development|PrintString "Healed" true true "(R=1.000000,G=0.000000,B=0.062871,A=1.000000)")
  (if (> (+ Amount%20Healed (Variables|Default|GetCurrent%20HP)) (Variables|Default|GetMax%20HP))
    (Variables|Default|SetCurrent%20HP (Variables|Default|GetMax%20HP))
    (else
      (Variables|Default|SetCurrent%20HP (+ Amount%20Healed (Variables|Default|GetCurrent%20HP)))))
  (CallFunction|UpdateScreen (Variables|Default|GetCurrent%20HP)))

(event EventTick
  (params (DeltaSeconds :type Float%20%28single-precision%29))
  (if (Variables|Default|GetShell%20Applied?)
    (if (>= (Variables|Default|GetShell%20Duration) 0)
      (Variables|Default|SetShell%20Duration (- (Variables|Default|GetShell%20Duration) 10))
      (else
        (Variables|Default|SetShell%20Applied? false))))
  (CallFunction|ApplyRegen)
  (CallFunction|ApplyHaste/Slow)
  (Utilities|FlowControl|Gate false :!label _label
    (:Exit
      (Development|PrintString "Enter" true true "(R=0.000000,G=0.660000,B=1.000000,A=1.000000)" 0.005)
      (if (< (Variables|Default|GetCurrent%20Filled) (Variables|Default|GetPlayer%20Speed))
        (bind _output_get (Variables|Default|SetCurrent%20Filled (+ (Variables|Default|GetCurrent%20Filled) (Variables|Default|GetRate%20ATB%20Increases))))
        (CallFunction|SetFillonScreenATB _output_get)
        (return)
        (else
          (Development|PrintString "Notify ATB Full")
          (CallFunction|NotifyATBFull)
          (goto _label Close))))))

(fn ConstructionScript)

(fn SetFillonScreenATB
  (params (CurrentFilled :type Float%20%28double-precision%29)))

(fn NotifyATBFull)

(fn ApplyHaste/Slow
  (if (or (Variables|Default|GetHaste%20Enabled?) (Variables|Default|GetSlow%20Enabled?))
    (if (<= (Variables|Default|GetLength%20Of%20Haste) 0)
      (Variables|Default|SetHaste%20Enabled? false)
      (Variables|Default|SetSlow%20Enabled? false)
      (Variables|Default|SetRate%20ATB%20Increases (/ (Variables|Default|GetRate%20ATB%20Increases) 2.0))
      (else
        (Variables|Default|SetLength%20Of%20Haste (- (Variables|Default|GetLength%20Of%20Haste) 10))))))

(fn ApplyRegen
  (bind _regen_frequency (Variables|Default|GetRegen%20Frequency))
  (if (Variables|Default|GetRegen%20Enabled?)
    (Development|PrintString "Regen" true true "(R=0.000000,G=0.660000,B=1.000000,A=1.000000)" 0.0005)
    (if (>= (Variables|Default|GetLength%20of%20Regen) 0)
      (Variables|Default|SetLength%20of%20Regen (- (Variables|Default|GetLength%20of%20Regen) 10))
      (if (> _regen_frequency (Variables|Default|GetTime%20to%20Next%20Regen))
        (Variables|Default|SetTime%20to%20Next%20Regen (+ (Variables|Default|GetTime%20to%20Next%20Regen) 10))
        (Development|PrintString (Utilities|String|Append "Time to Next Regen:" (Utilities|String|ToString(Integer) (- _regen_frequency (+ (Variables|Default|GetTime%20to%20Next%20Regen) 10)))) true true "(R=0.000000,G=0.660000,B=1.000000,A=1.000000)" 0.0005)
        (else
          (CallFunction|Healed (/ (Variables|Default|GetMax%20HP) 16) false)
          (Variables|Default|SetTime%20to%20Next%20Regen 0)))
      (else
        (Variables|Default|SetHaste%20Enabled? false)))))

(fn UpdateScreen
  (params (HP :type Integer) (MP :type Integer)))