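; BP_Dagger is a JRPG battle character that adds White Magic spell selection to its parent's behavior.
; On BeginPlay it creates a hidden spells menu for White Magic, which the command widget's unique button reveals.
; All spell buttons share one event that queues a spell name, sets the action, notifies the battle game mode and hides the menu.
; That event reads the name from the binding loop's cast reference, not the pressed button.
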(event `self.ReceiveBeginPlay`
  (`parent.ReceiveBeginPlay`)
  (bind _returnvalue (`|CreateWidget` "/Game/Blueprints/Widgets/BattleMenu/WBP_SpellsMenu.WBP_SpellsMenu_C"))
  (`/Game/Blueprints/Widgets/BattleMenu/WBP_SpellsMenu.Init_SpellsMenu` _returnvalue "/Game/Data/WhiteMagic.WhiteMagic")
  (`UserWidget.AddToViewport` _returnvalue 0)
  (`Widget.SetVisibility` _returnvalue "Hidden")
  (add `Button.OnPressed` (`/Game/Blueprints/Widgets/BattleMenu/WBP_IndividualCommand.Button` (`/Game/Blueprints/Widgets/BattleMenu/WBP_Commands.Unique` (`self.CommandsWidget`))) (delegate `WhiteMagicBtnEvent`))
  (for _array_element (`PanelWidget.GetAllChildren` (`/Game/Blueprints/Widgets/BattleMenu/WBP_SpellsMenu.ScrollBox_9` _returnvalue))
    (bind _aswbp_individual_spells (cast `/Game/Blueprints/Widgets/BattleMenu/WBP_IndividualSpells` _array_element))
    (add `Button.OnPressed` (`/Game/Blueprints/Widgets/BattleMenu/WBP_IndividualSpells.Button_10` _aswbp_individual_spells) (delegate `Spell Selected`))))

(event `Spell Selected`
  (set `self.SpellQueued` (`/Game/Blueprints/Widgets/BattleMenu/WBP_IndividualSpells.Name_Spell` (stale `self.ReceiveBeginPlay` _aswbp_individual_spells)))
  (set `self.Action` "NewEnumerator11")
  (`/Game/GameMode_JRPGBattle.Action Added` (`self.As Game Mode JRPGBattle`) self)
  (`Widget.SetVisibility` (stale `self.ReceiveBeginPlay` _returnvalue) "Hidden"))

(event `WhiteMagicBtnEvent`
  (`Widget.SetVisibility` (stale `self.ReceiveBeginPlay` _returnvalue) "Visible"))

(fn `UserConstructionScript`
  (`parent.UserConstructionScript`))