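; Playable party-member base for an ATB JRPG battle, with Final Fantasy IX-style stats, damage formulas and spells.
; A full ATB gauge notifies the game mode, or auto-queues Attack under Berserk; the Attack button opens target selection.
; PerformAction dispatches the chosen action to attack, steal, data-table black magic, summon or white magic functions.
; Many results are only printed, and several white magic calls pass placeholder inputs.
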(event `self.ReceiveBeginPlay`
  (bind _asgame_mode_jrpgbattle (cast `/Game/GameMode_JRPGBattle` (`GameplayStatics.GetGameMode`)))
  (set `self.As Game Mode JRPGBattle` _asgame_mode_jrpgbattle)
  (`self.SetupCommandsMenu`)
  (add `Button.OnPressed` (`/Game/Blueprints/Widgets/BattleMenu/WBP_IndividualCommand.Button` (`/Game/Blueprints/Widgets/BattleMenu/WBP_Commands.Attack` (`self.CommandsWidget`))) (delegate `AttackOnPressedEvent`)))

(event `AttackOnPressedEvent`
  (set `self.Action` "NewEnumerator0")
  (`Widget.SetVisibility` (`self.CommandsWidget`) "Hidden")
  (`Widget.SetVisibility` (`/Game/GameMode_JRPGBattle.Select Target` (`self.As Game Mode JRPGBattle`)) "Visible"))

(event `Target Selected`
  (`/Game/GameMode_JRPGBattle.Action Added` (`self.As Game Mode JRPGBattle`) self))

(event `self.ReceiveTick`
  (params (DeltaSeconds :type "Float (single-precision)"))
  (`parent.ReceiveTick` 0.0))

(event `Damage Taken`
  (params (`Amount Taken` :type Integer) (`Magical Damage` :type Boolean))
  (set `self.Current HP` (- (`self.Current HP`) `Amount Taken`))
  (`KismetSystemLibrary.PrintString` (`KismetStringLibrary.Concat_StrStr` "Damage Taken::" (`KismetStringLibrary.Conv_IntToString` `Amount Taken`) " \nBy ::" (`KismetSystemLibrary.GetDisplayName` self)))
  (`/Game/Blueprints/Widgets/BattleMenu/WBP_UniqueBattleStatScreen.UpdateHP/MP` (`self.UniqueBattleStatScreen`) (`KismetTextLibrary.Conv_IntToText` (`self.Current HP`)) (`KismetTextLibrary.Conv_IntToText` (`self.MP`))))

(event `Perform Action`
  (`self.RunCorrectEvent`))

(fn `Cast Beserk`
  (params (`Target's Level` :type Integer) (`Target's Magic Evade` :type Integer))
  (locals (Chance :type Integer))
  (if (not (`self.Beserk Enabled?`))
    (set `local.Chance` (- (+ 75 (`self.Level`) (/ (`self.Magic`) 4)) (`local.Target's Level`)))
    (if (>= (`KismetMathLibrary.RandomIntegerInRange` 0 99) (`local.Chance`))
      (`KismetSystemLibrary.PrintString` "Beserk Missed")
      (elif (< (`local.Chance`) (`local.Target's Magic Evade`))
        (`KismetSystemLibrary.PrintString` "The target evaded Beserk")
        (else
          (set `self.Beserk Enabled?` false))))
    (else
      (`KismetSystemLibrary.PrintString` "Beserk Already On"))))

(fn `Cast Confuse`
  (params (`Target's Level` :type Integer) (`Target's Magic Evade` :type Integer))
  (locals (Chance :type Integer))
  (if (not (`self.Confuse Enabled?`))
    (set `local.Chance` 0)
    (if (>= (`KismetMathLibrary.RandomIntegerInRange` 0 99) (`local.Chance`))
      (`KismetSystemLibrary.PrintString` "Confuse Missed")
      (elif (< (`local.Chance`) (`local.Target's Magic Evade`))
        (`KismetSystemLibrary.PrintString` "The target evaded Confuse")
        (else
          (set `self.Confuse Enabled?` true))))
    (else
      (`KismetSystemLibrary.PrintString` "Can't Cast. Confuse already affected"))))

(fn `Cast Haste`
  (if (not (`self.Haste Enabled?`))
    ;[1 1 1] Change Boolean
    (set `self.Haste Enabled?` true)
    ;[1 1 1] Increase Rate of Haste
    (set `self.Rate ATB Increases` (* (`self.Rate ATB Increases`) 2.0))
    (if (`self.Slow Enabled?`)
      (set `self.Length Of Haste` 0)
      (else
        ;[1 1 1] Set Length of Effect
        (set `self.Length Of Haste` (* (`self.Spirit`) 320))))
    (else
      (`KismetSystemLibrary.PrintString` "Failed as Haste is Already Enabled"))))

(fn `Cast Life`
  (params (`Targets Life` :type Integer) (`Targets Magic Evasion` :type Integer) (`Full-Life?` :type Boolean))
  (if (`self.Dead?`)
    (if `Full-Life?`
      (`self.Healed` (`self.Max HP`) true)
      (else
        ;[1 1 1] Amount
        (`self.Healed` (* (+ (`self.Spirit`) 5) (/ (`self.Max HP`) 100)) true)))
    (else
      (`KismetSystemLibrary.PrintString` "Failed to Cast Life as the target is Alive"))))

(fn `Cast Mini`
  (params (`Target's Level` :type Integer) (`Target's Magic Evade` :type Integer))
  (locals (Chance :type Integer))
  (if (not (`self.Mini Enabled?`))
    (set `local.Chance` (- (+ 50 (`self.Level`) (/ (`self.Magic`) 4)) (`local.Target's Level`)))
    (if (>= (`KismetMathLibrary.RandomIntegerInRange` 0 99) (`local.Chance`))
      (`KismetSystemLibrary.PrintString` "Mini Missed")
      (elif (< (`local.Chance`) (`local.Target's Magic Evade`))
        (`KismetSystemLibrary.PrintString` "The target evaded Mini")
        (else
          (set `self.Mini Enabled?` true))))
    (else
      (`KismetSystemLibrary.PrintString` "Can't Apply mini, target is already affected"))))

(fn `Cast Regen`
  (if (not (`self.Regen Enabled?`))
    ;[1 1 1] Change Boolean
    (set `self.Regen Enabled?` true)
    ;[1 1 1] Heal Frequency
    (set `self.Regen Frequency` (* (- 60 (`self.Spirit`)) 40))
    ;[1 1 1] Set Length of Effect
    (set `self.Length of Regen` (* (`self.Spirit`) 360))
    (else
      (`KismetSystemLibrary.PrintString` "Failed to Cast Regen as it is already applied"))))

(fn `Cast Scan`
  (params (`Scan Target` :type "/Game/Blueprints/BattleCharacter Object Reference"))
  ;[1 1 1] Is Enemy Heavy?
  (if (not false)
    (`KismetSystemLibrary.PrintString` (`KismetSystemLibrary.GetDisplayName` `Scan Target`))
    (`KismetSystemLibrary.PrintString` (`KismetStringLibrary.Conv_IntToString` (`/Game/Blueprints/BattleCharacter.Current HP` (`local.Scan Target`))))
    (else
      (`KismetSystemLibrary.PrintString` "Can't Scan Enemy"))))

(fn `Cast Shell`
  (if (not (`self.Shell Applied?`))
    (set `self.Shell Duration` (* (`self.Spirit`) 360))
    (set `self.Shell Applied?` true)
    (else
      (`KismetSystemLibrary.PrintString` "Cannot apply Shell, already applied to target"))))

(fn `Cast Silence`
  (params (`Target's Level` :type Integer) (`Target's Magic Evasion` :type Integer))
  (locals (Chance :type Integer))
  (if (not (`self.Silence Enabled?`))
    (if (`KismetMathLibrary.RandomBoolWithWeight` 0.5)
      (set `local.Chance` (- (+ 50 (`self.Level`) (/ (`self.Magic`) 4)) (`local.Target's Level`)))
      (if (>= (`KismetMathLibrary.RandomIntegerInRange` 0 99) (`local.Chance`))
        (`KismetSystemLibrary.PrintString` "Silence Misses")
        (elif (< (`local.Chance`) (`local.Target's Magic Evasion`))
          (`KismetSystemLibrary.PrintString` "Silence Evaded")
          (else
            (set `self.Shell Applied?` true))))
      (else
        (`KismetSystemLibrary.PrintString` "Missed")))
    (else
      (`KismetSystemLibrary.PrintString` "Can't cast Silence, target already is affected"))))

(fn `Cast Slow`
  (if (not (`self.Slow Enabled?`))
    ;[1 1 1] Change Boolean
    (set `self.Slow Enabled?` true)
    ;[1 1 1] Increase Rate of Haste
    (set `self.Rate ATB Increases` (* (`self.Rate ATB Increases`) 0.5))
    (if (`self.Haste Enabled?`)
      (set `self.Length Of Haste` 0)
      (else
        ;[1 1 1] Set Length of Effect
        (set `self.Length Of Haste` (* (`self.Spirit`) 320))))
    (else
      (`KismetSystemLibrary.PrintString` "Failed as Haste is Already Enabled"))))

(fn `Get Black Magic Damage`
  (params (TargetMagicDefence :type Integer))
  (returns (NewParam :type Integer))
  (bind _returnvalue (`|GetDataTableRow` "/Game/Data/BlackMagic.BlackMagic" (`self.SpellQueued`))
    (:`then`
      (`self.CheckMP` (`.MP_17_604564164298EE252A37AB9BF4A155C1` (break `/Game/Data/Spells` _returnvalue)))
      (set `self.MP` (- (`self.MP`) (`.MP_17_604564164298EE252A37AB9BF4A155C1` (break `/Game/Data/Spells` _returnvalue))))
      (return (* (- (`.SpellPower_18_F943C5F748EC9C2C888C38BECC8CED1D` (break `/Game/Data/Spells` _returnvalue)) TargetMagicDefence) (+ (`self.Magic`) (mod (`KismetMathLibrary.RandomIntegerInRange` 0 255) (+ (/ (+ (`self.Level`) (`self.Magic`)) 8) 1))))))))

(fn `Get Healing Amount`
  (params (`Base Spell Power` :type Integer))
  (`KismetSystemLibrary.PrintString` (`KismetStringLibrary.Conv_IntToString` (* `Base Spell Power` (+ (`self.Magic`) (mod (`KismetMathLibrary.RandomIntegerInRange` 0 255) (+ (/ (+ (`self.Level`) (`self.Magic`)) 8) 1)))))))

(fn `Get Physical Attack Damage`
  (params (`Target Defence` :type Integer) (`Target Modifer` :type Integer :default 1))
  (locals (Base :type Integer) (Bonus :type Integer))
  (bind _returnvalue (+ (mod (`KismetMathLibrary.RandomIntegerInRange` 0 255) (+ (/ (+ (`self.Strength`) (`self.Level`)) 8) 1)) (`self.Strength`)))
  ;[1 1 1] Damage = Base (Strength - Defence) * Bonus(Strength + Rnd (0...255) Modulo ((Level_Strength)/8 + 1))) * Modifier (Enemy Resistance)
  (set `local.Base` (- (`self.Power`) `Target Defence`))
  (if (`self.Beserk Enabled?`)
    (set `local.Bonus` (/ (* _returnvalue 3) 2))
    (else
      (set `local.Bonus` _returnvalue)))
  (`KismetSystemLibrary.PrintString` (`KismetStringLibrary.Conv_IntToString` (* (* (`local.Base`) (`local.Bonus`)) `Target Modifer`))))

(fn `Get Steal`
  (params (`Target Level` :type Integer))
  (locals (StealOdds :type "Array of Integer"))
  (bind _output (`|GetArrayItem` (`self.BP_Enemy`)))
  ;[1 1 1] True Steal Sucseeds
  (if (>= (`KismetMathLibrary.RandomIntegerInRange` 0 (- (+ (`self.Level`) (`self.Spirit`)) 1)) (`KismetMathLibrary.RandomIntegerInRange` 0 (- `Target Level` 1)))
    (for (_array_element _array_index) (`|MakeArray` (`/Game/Blueprints/BP_Enemy.Steal Very Rare` _output) (`/Game/Blueprints/BP_Enemy.Steal Rare` _output) (`/Game/Blueprints/BP_Enemy.Steal Uncommon` _output) (`/Game/Blueprints/BP_Enemy.Steal Common` _output))
      (if (<= (`KismetMathLibrary.RandomIntegerInRange` 1 256) (`|GetArrayItem` (`local.StealOdds`) _array_index))
        (if (!= _array_element "None")
          (`KismetSystemLibrary.PrintString` (`KismetStringLibrary.Concat_StrStr` "Zidane Stole::" (`KismetStringLibrary.Conv_NameToString` _array_element)))
          (break)
          (else
            (`KismetSystemLibrary.PrintString` "Zidane: The Enemy hadNothing To Steal")))))
    (else
      (`KismetSystemLibrary.PrintString` "Zadine Failed to Steal"))))

(fn `GetSummon Damage`
  (params (`Summon MP Cost` :type Integer) (`Summon Power` :type Integer) (`Target Magic Def` :type Integer))
  (bind _returnvalue (* (- (`local.Summon Power`) (`local.Target Magic Def`)) (mod (`KismetMathLibrary.RandomIntegerInRange` 0 255) (+ (/ (+ (`self.Level`) (`self.Magic`)) 8) 1))))
  ;[1 1 1] Determines Odds of Full Animation
  (if (< (`self.MP`) (* `Summon MP Cost` 2))
    ;[1 1 1] True in Either leads to Full Animations
    (if (>= (mod (`KismetMathLibrary.RandomIntegerInRange` 0 255) 256) 170)
      (`KismetSystemLibrary.PrintString` (`KismetStringLibrary.Concat_StrStr` "Full Anim::" (`KismetStringLibrary.Conv_IntToString` _returnvalue)) :!label _label)
      (else
        (`KismetSystemLibrary.PrintString` (`KismetStringLibrary.Concat_StrStr` "Half Anim::" (`KismetStringLibrary.Conv_IntToString` (/ (* _returnvalue 2) 3))) :!label _label_2)))
    (elif (>= (mod (`KismetMathLibrary.RandomIntegerInRange` 0 255) 256) 230)
      (goto _label)
      (else
        (goto _label_2)))))

(fn `NotifyATBFull`
  (`parent.NotifyATBFull`)
  (if (`self.Beserk Enabled?`)
    (set `self.Action` "NewEnumerator0")
    (`/Game/GameMode_JRPGBattle.Action Added` (`self.As Game Mode JRPGBattle`) self)
    (else
      (`/Game/GameMode_JRPGBattle.Main Character ATB Filled` (`self.As Game Mode JRPGBattle`) self))))

(fn `RunCorrectEvent`
  (switch `/Game/Blueprints/ActionsAbilities` (`self.Action`)
    (:`NewEnumerator0`
      (`self.Get Physical Attack Damage` (`/Game/Blueprints/BattleCharacter.Defense` (`self.CurrentAbilityTarget`)))
      (`/Game/GameMode_JRPGBattle.Action End` (`self.As Game Mode JRPGBattle`) false :!label _label))
    (:`NewEnumerator4`
      (`self.Get Steal` (`/Game/Blueprints/BattleCharacter.Level` (`self.CurrentAbilityTarget`)))
      (goto _label))
    (:`NewEnumerator6`
      (`self.Get Black Magic Damage` (`/Game/Blueprints/BattleCharacter.Mag Def` (`self.CurrentAbilityTarget`)))
      (goto _label))
    (:`NewEnumerator9`
      (`self.GetSummon Damage` 0))
    (:`NewEnumerator11`
      (`self.White Magic Spell Select`)
      (goto _label))))

(fn `Set Guage Length`
  (returns (Init :type Integer) (`StartingATB Filled` :type "Float (double-precision)"))
  (bind _returnvalue (* (- 60 (`self.Speed`)) 160))
  (bind _returnvalue_2 (/ _returnvalue 4))
  (return _returnvalue (`KismetMathLibrary.Conv_IntToDouble` (`KismetMathLibrary.RandomIntegerInRange` _returnvalue_2 (* _returnvalue_2 3)))))

(fn `SetFillOnScreenATB`
  (params (CurrentFilled :type "Float (double-precision)"))
  (`parent.SetFillOnScreenATB` CurrentFilled)
  (`ProgressBar.SetPercent` (`/Game/Blueprints/Widgets/BattleMenu/WBP_UniqueBattleStatScreen.ATB_ProgressBar` (`self.UniqueBattleStatScreen`)) (/ CurrentFilled (`self.Player Speed`))))

(fn `SetInitStats`
  (params (`Character Sheet` :type "DataTable Object Reference") (`Battle Character` :type "/Game/Blueprints/Widgets/BattleMenu/WBP_UniqueBattleStatScreen Object Reference"))
  (bind _returnvalue (`KismetTextLibrary.Conv_IntToText` (`self.Current HP`)))
  (bind _returnvalue_2 (`KismetTextLibrary.Conv_IntToText` (`self.MP`)))
  (bind _output_get (set `self.UniqueBattleStatScreen` `Battle Character`))
  (`TextBlock.SetText` (`/Game/Blueprints/Widgets/BattleMenu/WBP_UniqueBattleStatScreen.CurrentHP` _output_get) _returnvalue)
  (`TextBlock.SetText` (`/Game/Blueprints/Widgets/BattleMenu/WBP_UniqueBattleStatScreen.MaxHP` _output_get) _returnvalue)
  (`TextBlock.SetText` (`/Game/Blueprints/Widgets/BattleMenu/WBP_UniqueBattleStatScreen.CurrentMP` _output_get) _returnvalue_2)
  (`TextBlock.SetText` (`/Game/Blueprints/Widgets/BattleMenu/WBP_UniqueBattleStatScreen.MaxMP` _output_get) _returnvalue_2))

(fn `SetupCommandsMenu`
  (bind _returnvalue (`|CreateWidget` "/Game/Blueprints/Widgets/BattleMenu/WBP_Commands.WBP_Commands_C"))
  (set `self.CommandsWidget` _returnvalue)
  (`UserWidget.AddToViewport` _returnvalue 0)
  (for (_array_element _array_index) (`|MakeArray` (`/Game/Blueprints/Widgets/BattleMenu/WBP_Commands.Unique` _returnvalue) (`/Game/Blueprints/Widgets/BattleMenu/WBP_Commands.Unique_1` _returnvalue))
    (`TextBlock.SetText` (`/Game/Blueprints/Widgets/BattleMenu/WBP_IndividualCommand.CommandName` _array_element) (`|GetArrayItem` (`self.UniqueAbilities`) _array_index))))

(fn `Update Screen`
  (params (HP :type Integer) (MP :type Integer))
  (`/Game/Blueprints/Widgets/BattleMenu/WBP_UniqueBattleStatScreen.UpdateHP/MP` (`self.UniqueBattleStatScreen`) (`KismetTextLibrary.Conv_IntToText` HP) (`KismetTextLibrary.Conv_IntToText` MP)))

(fn `UserConstructionScript`)

(fn `White Magic Spell Select`
  (switch `name` (`self.SpellQueued`)
    (:`Default`
      (`self.Get Healing Amount` 0))
    (:`Regen`
      (`self.Cast Regen`))
    (:`Life`
      (`self.Cast Life` 0))
    (:`Full Life`
      (`self.Cast Life` 0 0 true))
    (:`Scan`
      (`self.Cast Scan` null))
    (:`Shell`
      (`self.Cast Shell`))
    (:`Haste`
      (`self.Cast Haste`))
    (:`Silence`
      (`self.Cast Silence` 0))
    (:`Mini`
      (`self.Cast Mini` 0))
    (:`Confuse`
      (`self.Cast Confuse` 0))
    (:`Beserk`
      (`self.Cast Beserk` 0))))