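; BP_Zidane is a playable battle character for a JRPG battle mode, with Steal as its unique command.
; On BeginPlay it runs the parent logic, then binds the unique button in its commands widget to a steal event.
; Pressing that button sets the character's action enum and notifies the JRPG battle game mode that an action was added.
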(event `self.ReceiveBeginPlay`
  (`parent.ReceiveBeginPlay`)
  (add `Button.OnPressed` (`/Game/Blueprints/Widgets/BattleMenu/WBP_IndividualCommand.Button` (`/Game/Blueprints/Widgets/BattleMenu/WBP_Commands.Unique` (`self.CommandsWidget`))) (delegate `StealButtonEvent`)))

(event `StealButtonEvent`
  (set `self.Action` "NewEnumerator4")
  (`/Game/GameMode_JRPGBattle.Action Added` (`self.As Game Mode JRPGBattle`) self))

(fn `UserConstructionScript`
  (`parent.UserConstructionScript`))