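; BP_Enemy is an enemy combatant in an ATB-style JRPG battle, driven by the JRPG battle game mode.
; It caches the game mode on BeginPlay and, when notified its ATB is full, calls the parent logic and adds itself to the action queue.
; EnemyAttackCalculation deals fixed physical damage from the placeholder DemoAttack function to a random party member, then signals the game mode that the action has ended.
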(event `self.ReceiveBeginPlay`
  (bind _asgame_mode_jrpgbattle (cast `/Game/GameMode_JRPGBattle` (`GameplayStatics.GetGameMode`)))
  (set `self.As Game Mode JRPGBattle` _asgame_mode_jrpgbattle))

(event `self.ReceiveTick`
  (params (DeltaSeconds :type "Float (single-precision)"))
  (`parent.ReceiveTick` 0.0))

(event `Enemy Attack Calculation`
  (bind _as_game_mode_jrpgbattle (`self.As Game Mode JRPGBattle`))
  (bind _damage_dealth (`self.DemoAttack`))
  (`/Game/Blueprints/BP_MainCharacters.Damage Taken` (`KismetArrayLibrary.Array_Random` (`/Game/GameMode_JRPGBattle.Party` _as_game_mode_jrpgbattle)) _damage_dealth false)
  (`/Game/GameMode_JRPGBattle.Action End` _as_game_mode_jrpgbattle true))

(fn `DemoAttack`
  (returns (`Damage Dealth` :type Integer))
  (return 10))

(fn `NotifyATBFull`
  (`parent.NotifyATBFull`)
  (`/Game/GameMode_JRPGBattle.Enemy Adds to Queue` (`self.As Game Mode JRPGBattle`) self))

(fn `UserConstructionScript`)